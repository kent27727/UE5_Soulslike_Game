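; Base Blueprint for dual-wielded weapons, extending a parent weapon with an off-hand mesh and right-foot hit detection on the owning character.
; Equipping binds collision components to both meshes, ignores the owner and attaches the off-hand weapon to a hand or stow socket, which follows combat toggles.
; Collision is switched per part (main, off-hand, foot); off-hand and foot hits apply point damage to actors accepting damage.
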(event `self.ToggleCombat`
  (params (`bEnableCombat?` :type Boolean))
  (`parent.ToggleCombat` `bEnableCombat?`)
  (`self.AttachOff-HandWeapon` (select `bool` `bEnableCombat?` :`false` (`self.Second Weapon Attach Socket`) :`true` (`self.Second Weapon Hand Socket`))))

(event `self.Off-HandWeaponCollisionComponent.OnHit`
  (params (HitResult :type "HitResult Structure"))
  (bind (_bblockinghit _binitialoverlap _time _distance _location _impactpoint _normal _impactnormal _physmat _hitactor) (`GameplayStatics.BreakHitResult` HitResult))
  (bind _returnvalue (message `/Game/CombatSystem/Blueprints/Interfaces/Combat_BPI.CanRecieveDamage` _hitactor))
  (if _returnvalue
    (`GameplayStatics.ApplyPointDamage` _hitactor (`self.GetDamage`) (`self.GetActorForwardVector` (`self.GetOwner`)) HitResult (`self.GetInstigatorController`) self)))

(event `self.BP_RighFoot.OnHit`
  (params (HitResult :type "HitResult Structure"))
  (bind (_bblockinghit _binitialoverlap _time _distance _location _impactpoint _normal _impactnormal _physmat _hitactor) (`GameplayStatics.BreakHitResult` HitResult))
  (bind _returnvalue (message `/Game/CombatSystem/Blueprints/Interfaces/Combat_BPI.CanRecieveDamage` _hitactor))
  (if _returnvalue
    (`GameplayStatics.ApplyPointDamage` _hitactor (`self.GetDamage`) (`self.GetActorForwardVector` (`self.GetOwner`)) HitResult (`self.GetInstigatorController`) self)))

(fn `ActivateCollision`
  (params (CollisionPart :type "/Game/CombatSystem/Blueprints/Enums/E_CollisionPart Enum" :default "NewEnumerator0"))
  (switch `/Game/CombatSystem/Blueprints/Enums/E_CollisionPart` CollisionPart
    (:`NewEnumerator0`
      (`/Game/CombatSystem/Blueprints/Components/BP_CollisionComponent.Activate Collision` (`self.MainWeaponCollisionComponent`)))
    (:`NewEnumerator1`
      (`/Game/CombatSystem/Blueprints/Components/BP_CollisionComponent.Activate Collision` (`self.Off-HandWeaponCollisionComponent`)))
    (:`NewEnumerator2`
      (`/Game/CombatSystem/Blueprints/Components/BP_CollisionComponent.Activate Collision` (`self.BP_RighFoot`)))))

(fn `AttachOff-HandWeapon`
  (params (Socket :type Name))
  (`SceneComponent.K2_AttachToComponent` (`self.Off-HandWeaponMesh`) (`Character.Mesh` (cast `Character` (`self.GetOwner`) :!pure true)) Socket "SnapToTarget" "SnapToTarget" "SnapToTarget" true))

(fn `Deactivate Collision`
  (params (CollisionPart :type "/Game/CombatSystem/Blueprints/Enums/E_CollisionPart Enum" :default "NewEnumerator0"))
  (switch `/Game/CombatSystem/Blueprints/Enums/E_CollisionPart` CollisionPart
    (:`NewEnumerator0`
      (`/Game/CombatSystem/Blueprints/Components/BP_CollisionComponent.Deactivate Collision` (`self.MainWeaponCollisionComponent`)))
    (:`NewEnumerator1`
      (`/Game/CombatSystem/Blueprints/Components/BP_CollisionComponent.Deactivate Collision` (`self.Off-HandWeaponCollisionComponent`)))
    (:`NewEnumerator2`
      (`/Game/CombatSystem/Blueprints/Components/BP_CollisionComponent.Deactivate Collision` (`self.BP_RighFoot`)))))

(fn `OnEquipped`
  (`parent.OnEquipped`)
  (`/Game/CombatSystem/Blueprints/Components/BP_CollisionComponent.SetCollisionMesh` (`self.Off-HandWeaponCollisionComponent`) (`self.Off-HandWeaponMesh`))
  (`/Game/CombatSystem/Blueprints/Components/BP_CollisionComponent.SetCollisionMesh` (`self.BP_RighFoot`) (`Character.Mesh` (cast `Character` (`self.GetOwner`) :!pure true)))
  (`self.AttachOff-HandWeapon` (select `bool` (`/Game/CombatSystem/Blueprints/Components/BP_CombatComponent.Is Combat Enabled?` (`self.CombatCombatComponent`)) :`false` (`self.Second Weapon Attach Socket`) :`true` (`self.Second Weapon Hand Socket`)))
  (`/Game/CombatSystem/Blueprints/Components/BP_CollisionComponent.AddActorToIgnore` (`self.BP_RighFoot`) (`self.GetOwner`))
  (`/Game/CombatSystem/Blueprints/Components/BP_CollisionComponent.AddActorToIgnore` (`self.Off-HandWeaponCollisionComponent`) (`self.GetOwner`)))

(fn `UserConstructionScript`
  (`parent.UserConstructionScript`))