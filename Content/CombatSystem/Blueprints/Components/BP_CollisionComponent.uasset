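; Actor component in the combat system that detects hits along a mesh by tracing between two sockets.
; While collision is enabled, Tick runs a multi-sphere object trace from the start socket to the end socket, skipping ignored actors.
; Each actor fires the OnHit dispatcher only once per activation, because hit actors are recorded and the list clears when collision is enabled again.
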(event `self.ReceiveTick`
  (params (DeltaSeconds :type "Float (single-precision)"))
  (if (`self.bIsCollisionEnabled?`)
    (`self.Collision Trace`)))

(event `SetCollisionMesh`
  (params (CollisionMeshComponent :type "PrimitiveComponent Object Reference"))
  ;[1 0 0.009134] Set Collision Mesh
  (set `self.CollisionMeshComponent` CollisionMeshComponent))

(event `Enable Collision`
  ;[1 0 0.009134] Enable Collision
  (`self.ClearHitActors`)
  (set `self.bIsCollisionEnabled?` true))

(event `Collision Trace`
  (bind _collisionmeshcomponent (`self.CollisionMeshComponent`))
  ;[1 0 0.009134] Collision Trace
  (bind _outhits (`KismetSystemLibrary.SphereTraceMultiForObjects` (`SceneComponent.GetSocketLocation` _collisionmeshcomponent (`self.Start Socket Name`)) (`SceneComponent.GetSocketLocation` _collisionmeshcomponent (`self.End Socket Name`)) (`self.TraceRadius`) (`self.Collision Object Types`) false (`self.Actors to Ignore`) (`self.Draw Debug Type`)))
  (for _array_element _outhits
    (bind _output_get (set `self.LastHit` _array_element))
    (bind (_bblockinghit _binitialoverlap _time _distance _location _impactpoint _normal _impactnormal _physmat _hitactor) (`GameplayStatics.BreakHitResult` _output_get))
    (if (not (`KismetArrayLibrary.Array_Contains` (`self.AlreadyHitActors`) _hitactor))
      (bind _output_get_2 (set `self.Hit Actor` _hitactor))
      (`KismetArrayLibrary.Array_Add` (`self.AlreadyHitActors`) _output_get_2)
      (`self.OnHit` (`self.LastHit`)))))

(event `Disable Collision`
  ;[1 0 0.009134] Disable Collision
  (set `self.bIsCollisionEnabled?` false))

(event `ClearHitActors`
  ;[1 0 0.009134] Clear Hit Actors
  (`KismetArrayLibrary.Array_Clear` (`self.AlreadyHitActors`)))

(fn `AddActorToIgnore`
  (params (InActor :type "Actor Object Reference (by ref)"))
  (`KismetArrayLibrary.Array_AddUnique` (`self.Actors to Ignore`) InActor))

(fn `GetActorToIgnore`
  (returns (ReturnValue :type "Array of Actor Object Reference"))
  (return (`self.Actors to Ignore`)))

(fn `GetAlreadyHitActors`
  (returns (ReturnValue :type "Array of Actor Object Reference"))
  (return (`self.AlreadyHitActors`)))

(fn `GetCollisionMeshComponent`
  (returns (ReturnValue :type "PrimitiveComponent Object Reference"))
  (return (`self.CollisionMeshComponent`)))

(fn `GetLastHit`
  (returns (ReturnValue :type "HitResult Structure"))
  (return (`self.LastHit`)))

(fn `IsCollisionEnabled?`
  (returns (ReturnValue :type Boolean))
  (return (`self.bIsCollisionEnabled?`)))

(fn `RemoveActorToIgnore`
  (params (InActorToRemove :type "Actor Object Reference (by ref)"))
  (`KismetArrayLibrary.Array_RemoveItem` (`self.Actors to Ignore`) InActorToRemove))